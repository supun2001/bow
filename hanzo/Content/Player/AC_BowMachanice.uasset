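; Player bow mechanics component that spawns a bow on the owning character's mesh socket and handles aiming, drawing and firing arrows.
; Aiming switches the character to controller-facing rotation and spawns a socketed arrow; ending aim restores movement and destroys it.
; A looping timer builds draw time, normalized into shot strength.
; Firing launches the arrow toward a camera line-trace target, plays a montage, then re-enters aim if still aiming.
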(event Custom|AimEnd
  (bind _character_ref (Variables|Character|GetCharacter%20Ref))
  (bind _charactermovement (Variables|/Script/Engine.Character|GetCharacterMovement _character_ref))
  ;[1 1 1] Aim ARrow
  (Variables|Aim|SetisAiming? false)
  (CallFunction|DrawEnd)
  (Variables|/Script/Engine.CharacterMovementComponent|SetbOrientRotationToMovement _charactermovement true)
  (Variables|/Script/Engine.CharacterMovementComponent|SetbUseControllerDesiredRotation _charactermovement false)
  (Variables|/Script/Engine.CharacterMovementComponent|SetRotationRate _charactermovement (Variables|Aim|GetInitialRotationRate))
  (Variables|/Game/Player/Wepons/BP_Bow.BP_Bow_C|SetBowState (Variables|Bow|GetBowRef) "NewEnumerator0")
  (CallFunction|DestroyArrow)
  (Default|CallOnAimEnd))

(event Custom|AimBegin
  (bind _character_ref (Variables|Character|GetCharacter%20Ref))
  (bind _charactermovement (Variables|/Script/Engine.Character|GetCharacterMovement _character_ref))
  ;[1 1 1] Aim ARrow
  (Variables|Aim|SetisAiming? true)
  (Variables|/Script/Engine.CharacterMovementComponent|SetbOrientRotationToMovement _charactermovement false)
  (Variables|/Script/Engine.CharacterMovementComponent|SetbUseControllerDesiredRotation _charactermovement true)
  (Variables|/Script/Engine.CharacterMovementComponent|SetRotationRate _charactermovement (Variables|Aim|GetAimRotationRate))
  (Variables|/Game/Player/Wepons/BP_Bow.BP_Bow_C|SetBowState (Variables|Bow|GetBowRef) "NewEnumerator1")
  (CallFunction|SpawnArrow)
  (Default|CallOnAimBegin))

(event Custom|FireArrowBegun
  ;[1 1 1] Fire Arrow
  (if (Variables|Draw|GetisDrawing?)
    (Variables|Draw|SetisFiringArrow true)
    (CallFunction|FireAimArrow)
    (CallFunction|DrawEnd)
    (Animation|Montage|PlayMontage (Variables|/Script/Engine.Character|GetMesh (Variables|Character|GetCharacter%20Ref)) (Variables|Draw|GetAimMontage)
      (:OnCompleted
        _)
      (:OnInterrupted
        _))
    (CallFunction|FireArrowEnd)))

(event Custom|DrawBegun
  ;[1 1 1] Drawing bow
  (Utilities|CanDrawBow
    (:Yes
      (Variables|Draw|SetisDrawing? true)
      (bind _returnvalue (Utilities|Time|SetTimerbyEvent (delegate Custom|IncrementDrawTimer) (Variables|Draw|GetDrawIncrementTimer) true))
      (Variables|Draw|SetDrawBowTime _returnvalue)
      (Default|DrawBegin (Variables|Bow|GetBowRef)))))

(event Custom|IncrementDrawTimer
  ;[1 1 1] Drawing bow
  (bind _output_get (Variables|Draw|SetDrawTime (+ (Variables|Draw|GetDrawTime) (Variables|Draw|GetDrawIncrementTimer))))
  (Development|PrintString (Utilities|String|ToString(Float) _output_get)))

(event Custom|DrawEnd
  ;[1 1 1] Drawing bow
  (Variables|Draw|SetisDrawing? false)
  (Variables|Draw|SetDrawTime 0.0)
  (Utilities|Time|ClearandInvalidateTimerbyHandle (Variables|Draw|GetDrawBowTime))
  (Default|DrawEnd (Variables|Bow|GetBowRef)))

(event Custom|FireArrowEnd
  ;[1 1 1] Fire Arrow
  (Variables|Draw|SetisFiringArrow false)
  (if (Variables|Aim|GetisAiming?)
    (CallFunction|AimBegin)))

(event EventBeginPlay
  (bind _ascharacter (Utilities|Casting|CastToCharacter (Components|GetOwner)))
  (Variables|Character|SetCharacter%20Ref _ascharacter)
  (CallFunction|EquipBow)
  (Variables|Aim|SetInitialRotationRate (Variables|/Script/Engine.CharacterMovementComponent|GetRotationRate (Variables|/Script/Engine.Character|GetCharacterMovement (Variables|Character|GetCharacter%20Ref)))))

(fn EquipBow
  (bind _returnvalue (Game|SpawnActorfromClass (Variables|Bow|GetBowClass) (Math|Transform|MakeTransform "0, 0, 0" "0, 0, 0" "1.000000,1.000000,1.000000") "Undefined" "MultiplyWithRoot" 0 0))
  (bind _output_get (Variables|Bow|SetBowRef _returnvalue))
  (Transformation|AttachComponentToComponent _output_get (Variables|/Script/Engine.Character|GetMesh (Variables|Character|GetCharacter%20Ref)) (Variables|Bow|GetBowSocketName) "KeepRelative" "KeepRelative" "KeepRelative" true))

(fn SpawnArrow
  (bind _returnvalue (Game|SpawnActorfromClass "/Game/Player/Wepons/BP_Arrow.BP_Arrow_C" (Math|Transform|MakeTransform "0, 0, 0" "0, 0, 0" "1.000000,1.000000,1.000000") "Undefined" "MultiplyWithRoot" 0 0))
  (bind _output_get (Variables|Arrow|SetArrowRef _returnvalue))
  (Transformation|AttachComponentToComponent _output_get (Variables|/Script/Engine.Character|GetMesh (Variables|Character|GetCharacter%20Ref)) (Variables|Arrow|GetArrowSocketName) "SnapToTarget" "SnapToTarget" "SnapToTarget" true))

(fn DestroyArrow
  (bind _arrowref (Variables|Arrow|GetArrowRef)
    (:then
      (Actor|DestroyActor _arrowref))
    (:else)))

(fn FireAimArrow
  (bind _arrowref (Variables|Arrow|GetArrowRef)
    (:then
      (Transformation|DetachFromActor _arrowref "KeepWorld" "KeepWorld" "KeepWorld")
      (bind _direction (CallFunction|CalculateAimDirection))
      (Default|Fire _arrowref _direction (Math|Float|Clamp(Float) (Math|Float|NormalizetoRange (Variables|Draw|GetDrawTime) 0.0 (Variables|/Game/Player/Wepons/BP_Bow.BP_Bow_C|GetMaxDrawTime (Variables|Bow|GetBowRef))))))
    (:else)))

(fn CalculateAimDirection
  (bind _character_ref (Variables|Character|GetCharacter%20Ref))
  (bind _returnvalue (Actor|GetComponentbyClass _character_ref "/Script/Engine.CameraComponent"))
  (bind _returnvalue_2 (Transformation|GetWorldLocation _returnvalue))
  (bind (_outhit _returnvalue_3) (Collision|LineTraceByChannel _returnvalue_2 (+ _returnvalue_2 (* (Math|Vector|GetForwardVector _returnvalue) 1e+04)) "TraceTypeQuery1" false 0 "Persistent"))
  (return (Math|Vector|GetUnitDirection(Vector) (Transformation|GetActorLocation (Variables|Arrow|GetArrowRef)) (Math|Vector|SelectVector (.Location (Collision|BreakHitResult _outhit)) (.TraceEnd (Collision|BreakHitResult _outhit)) _returnvalue_3))))